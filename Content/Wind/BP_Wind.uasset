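; Procedural wind actor that returns a wind vector for any world position via GetWindAt and writes scaled game time to MPC_Wind each tick.
; A random starting heading drifts on three sines, then varies by region, altitude and gust.
; GetGust sends layered sine waves downwind with a wavy front, lulls and punches.
; Speed combines gusts, ground shelter and regional variation, while gust rate of change adds vertical lift.
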(event EventTick
  (params (DeltaSeconds :type Float%20%28single-precision%29))
  (Rendering|Material|SetScalarParameterValue "/Game/Wind/MPC_Wind.MPC_Wind" "Time" (CallFunction|GetTime) :!class /Script/Engine.KismetMaterialLibrary))

(event EventBeginPlay
  (bind _output_get (Variables|Default|SetBaseDir (Math|Random|RandomFloatinRange 0.0 3.6e+02)))
  (Development|PrintText (Utilities|Text|FormatText "Starting Wind Dir: {n}" _output_get) true true "(R=0.416560,G=1.000000,B=0.000000,A=1.000000)" 1e+01))

(fn ConstructionScript)

(fn GetTime
  (return (* (Utilities|Time|GetTimeSeconds) (Variables|Default|GetTimeScale))))

(fn GetBaseDir
  (bind _seconds (CallFunction|GetTime))
  (bind _returnvalue (* _seconds 3.6e+02))
  (return (+ (Variables|Default|GetBaseDir) (* (Math|Trig|Sin(Degrees) (/ _returnvalue (Variables|Default|GetDriftPeriodA))) (Variables|Default|GetDriftAmpA)) (* (Math|Trig|Sin(Degrees) (/ _returnvalue (Variables|Default|GetDriftPeriodB))) (Variables|Default|GetDriftAmpB)) (* (Math|Trig|Sin(Degrees) (/ _returnvalue (Variables|Default|GetDriftPeriodC))) (Variables|Default|GetDriftAmpC)))))

(fn GetWindat
  (params (Pos :type Vector))
  (bind _regionspeedscale (Variables|Default|GetRegionSpeedScale))
  (bind _regionveer (Variables|Default|GetRegionVeer))
  (bind _groundz (Variables|Default|GetGroundZ))
  (bind _shelterheight (Variables|Default|GetShelterHeight))
  (bind _regionscale (Variables|Default|GetRegionScale))
  (bind _returnvalue (- (.z Pos) _groundz))
  (bind _returnvalue_2 (/ _returnvalue _shelterheight))
  (bind _returnvalue_3 (Math|Float|Clamp(Float) _returnvalue_2))
  (bind _returnvalue_4 (Math|Float|Lerp 0.5 1.0 _returnvalue_3))
  (LocalVariables|SetGust (CallFunction|GetGust Pos 0.0))
  (LocalVariables|SetGustPrev (CallFunction|GetGust Pos -0.4))
  (bind _output_get (LocalVariables|SetDir (CallFunction|GetBaseDir)))
  (return (+ (* (Math|Vector|GetForwardVector (Math|Rotator|MakeRotator 0.0 0.0 (+ _output_get (* (Math|Trig|Sin(Degrees) (/ (* (.x Pos) 3.6e+02) _regionscale)) _regionveer) (* _regionveer (Math|Trig|Sin(Degrees) (/ (* (.y Pos) 3.6e+02) (* _regionscale 1.37))) 0.7) (* (Math|Float|Clamp(Float) (/ _returnvalue (Variables|Default|GetVeerHeight))) (Variables|Default|GetAltitudeVeer)) (* (Variables|Gust|GetGustVeer) (- (LocalVariables|GetGust) 0.5) 2.0)))) (+ (Variables|Default|GetBaseSpeed) (* (Variables|Gust|GetGustSpeed) (LocalVariables|GetGust))) _returnvalue_4 (Math|Float|Lerp 0.2 1.0 (Math|Float|Clamp(Float) (+ (* (/ (+ (Math|Trig|Sin(Degrees) (/ (* (.x (- Pos (* (CallFunction|GetTime) (LocalVariables|GetDir) (Variables|Default|GetRegionSpeedSpeed)))) 3.6e+02) _regionspeedscale)) (Math|Trig|Sin(Degrees) (/ (* (.y (- Pos (* (CallFunction|GetTime) (LocalVariables|GetDir) (Variables|Default|GetRegionSpeedSpeed)))) 3.6e+02) (* _regionspeedscale 1.23))) (Math|Trig|Sin(Degrees) (/ (* (+ (.x (- Pos (* (CallFunction|GetTime) (LocalVariables|GetDir) (Variables|Default|GetRegionSpeedSpeed)))) (.y (- Pos (* (CallFunction|GetTime) (LocalVariables|GetDir) (Variables|Default|GetRegionSpeedSpeed))))) 3.6e+02 0.707) (* _regionspeedscale 0.81)))) 6.0) (Variables|Default|GetRegionSpeedContrast)) 0.5))) (Variables|Default|GetIntensityScale)) (Math|Vector|MakeVector 0.0 0.0 (* (Math|Float|Clamp(Float) (/ (/ (- (LocalVariables|GetGust) (LocalVariables|GetGustPrev)) 0.4) 1.0) -1.0) _returnvalue_4 (Variables|Default|GetGustLift) (Variables|Default|GetIntensityScale))))))

(fn GetGust
  (params (Pos :type Vector) (Offset :type Float%20%28double-precision%29))
  (bind _lullfloor (Variables|Gust|GetLullFloor))
  (LocalVariables|SetTemp (CallFunction|GetBaseDir))
  (return (Math|Float|Clamp(Float) (* (+ (Math|Float|Clamp(Float) (/ (- (Math|Float|Power (+ (* (+ (* (Math|Trig|Sin(Degrees) (/ (* (- (+ (CallFunction|GetTime) Offset) (/ (+ (Math|Vector|DotProduct Pos (Math|Vector|GetForwardVector (Math|Rotator|MakeRotator 0.0 0.0 (LocalVariables|GetTemp)))) (* (Math|Trig|Sin(Degrees) (* 3.6e+02 (/ (Math|Vector|DotProduct Pos (Math|Vector|GetForwardVector (Math|Rotator|MakeRotator 0.0 0.0 (+ (LocalVariables|GetTemp) 9e+01)))) 2.4e+04))) 4e+03)) (Variables|Gust|GetGustTravelSpeed))) 3.6e+02) (Variables|Gust|GetGustPeriodA))) (Variables|Gust|GetGustAmpA)) (* (Math|Trig|Sin(Degrees) (/ (* (- (+ (CallFunction|GetTime) Offset) (/ (+ (Math|Vector|DotProduct Pos (Math|Vector|GetForwardVector (Math|Rotator|MakeRotator 0.0 0.0 (LocalVariables|GetTemp)))) (* (Math|Trig|Sin(Degrees) (* 3.6e+02 (/ (Math|Vector|DotProduct Pos (Math|Vector|GetForwardVector (Math|Rotator|MakeRotator 0.0 0.0 (+ (LocalVariables|GetTemp) 9e+01)))) 2.4e+04))) 4e+03)) (Variables|Gust|GetGustTravelSpeed))) 3.6e+02) (Variables|Gust|GetGustPeriodB))) (Variables|Gust|GetGustAmpB)) (* (Math|Trig|Sin(Degrees) (/ (* (- (+ (CallFunction|GetTime) Offset) (/ (+ (Math|Vector|DotProduct Pos (Math|Vector|GetForwardVector (Math|Rotator|MakeRotator 0.0 0.0 (LocalVariables|GetTemp)))) (* (Math|Trig|Sin(Degrees) (* 3.6e+02 (/ (Math|Vector|DotProduct Pos (Math|Vector|GetForwardVector (Math|Rotator|MakeRotator 0.0 0.0 (+ (LocalVariables|GetTemp) 9e+01)))) 2.4e+04))) 4e+03)) (Variables|Gust|GetGustTravelSpeed))) 3.6e+02) (Variables|Gust|GetGustPeriodC))) (Variables|Gust|GetGustAmpC))) 0.5) 0.5) (Variables|Gust|GetGustBias)) _lullfloor) (- 1.0 _lullfloor))) (* (Math|Float|Power (Math|Float|Max(Float) (Math|Trig|Sin(Degrees) (/ (* (- (+ (CallFunction|GetTime) Offset) (/ (+ (Math|Vector|DotProduct Pos (Math|Vector|GetForwardVector (Math|Rotator|MakeRotator 0.0 0.0 (LocalVariables|GetTemp)))) (* (Math|Trig|Sin(Degrees) (* 3.6e+02 (/ (Math|Vector|DotProduct Pos (Math|Vector|GetForwardVector (Math|Rotator|MakeRotator 0.0 0.0 (+ (LocalVariables|GetTemp) 9e+01)))) 2.4e+04))) 4e+03)) (Variables|Gust|GetGustTravelSpeed))) 3.6e+02) (Variables|Gust|GetPunchPeriod))) 0.0) (Variables|Gust|GetPunchPower)) (Variables|Gust|GetPunchAmount))) (Math|Float|Lerp 0.2 1.2 (Math|Float|Power (+ (* (Math|Trig|Sin(Degrees) (/ (* (- (+ (CallFunction|GetTime) Offset) (/ (+ (Math|Vector|DotProduct Pos (Math|Vector|GetForwardVector (Math|Rotator|MakeRotator 0.0 0.0 (LocalVariables|GetTemp)))) (* (Math|Trig|Sin(Degrees) (* 3.6e+02 (/ (Math|Vector|DotProduct Pos (Math|Vector|GetForwardVector (Math|Rotator|MakeRotator 0.0 0.0 (+ (LocalVariables|GetTemp) 9e+01)))) 2.4e+04))) 4e+03)) (Variables|Gust|GetGustTravelSpeed))) 3.6e+02) 47.0)) 0.5) 0.5) 1.5))))))