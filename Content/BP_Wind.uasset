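; BP_Wind is a procedural wind field that returns a velocity vector for any world position through GetWindAt.
; Layered sines of scaled game time drift the base heading, which position-based regional veer, clamped altitude veer and gust veer then bend.
; GetGust sums travelling sine waves delayed along the base direction, adds sharpened punches and drives both speed and veer.
; Everything is computed on demand without stored state or Tick work.
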(event EventTick
  (params (DeltaSeconds :type Float%20%28single-precision%29)))

(fn ConstructionScript)

(fn GetTime
  (return (* (Utilities|Time|GetTimeSeconds) (Variables|Default|GetTimeScale))))

(fn GetBaseDir
  (bind _seconds (CallFunction|GetTime))
  (bind _returnvalue (* _seconds 3.6e+02))
  (return (+ (Variables|Default|GetBaseDir) (* (Math|Trig|Sin(Degrees) (/ _returnvalue (Variables|Default|GetDriftPeriodA))) (Variables|Default|GetDriftAmpA)) (* (Math|Trig|Sin(Degrees) (/ _returnvalue (Variables|Default|GetDriftPeriodB))) (Variables|Default|GetDriftAmpB)) (* (Math|Trig|Sin(Degrees) (/ _returnvalue (Variables|Default|GetDriftPeriodC))) (Variables|Default|GetDriftAmpC)))))

(fn GetWindat
  (params (Pos :type Vector))
  (bind _regionscale (Variables|Default|GetRegionScale))
  (bind _regionveer (Variables|Default|GetRegionVeer))
  (bind _dir (CallFunction|GetGust Pos))
  (return (* (Math|Vector|GetForwardVector (Math|Rotator|MakeRotator 0.0 0.0 (+ (CallFunction|GetBaseDir) (* (Math|Trig|Sin(Degrees) (/ (* (.x Pos) 3.6e+02) _regionscale)) _regionveer) (* _regionveer (Math|Trig|Sin(Degrees) (/ (* (.y Pos) 3.6e+02) (* _regionscale 1.37))) 0.7) (* (Math|Float|Clamp(Float) (/ (- (.z Pos) (Variables|Default|GetGroundZ)) (Variables|Default|GetVeerHeight))) (Variables|Default|GetAltitudeVeer)) (* (Variables|Gust|GetGustVeer) (- _dir 0.5) 2.0)))) (+ (Variables|Default|GetBaseSpeed) (* (Variables|Gust|GetGustSpeed) _dir)) (Variables|Default|GetIntensityScale))))

(fn GetGust
  (params (Pos :type Vector))
  (bind _seconds (CallFunction|GetTime))
  (bind _dir (CallFunction|GetBaseDir))
  (bind _gusttravelspeed (Variables|Gust|GetGustTravelSpeed))
  (bind _returnvalue (Math|Rotator|MakeRotator 0.0 0.0 _dir))
  (bind _returnvalue_2 (Math|Vector|GetForwardVector _returnvalue))
  (bind _returnvalue_3 (Math|Vector|DotProduct Pos _returnvalue_2))
  (bind _returnvalue_4 (/ _returnvalue_3 _gusttravelspeed))
  (bind _returnvalue_5 (- _seconds _returnvalue_4))
  (return (Math|Float|Clamp(Float) (+ (Math|Float|Power (+ (* (+ (* (Math|Trig|Sin(Degrees) (/ (* _returnvalue_5 3.6e+02) (Variables|Gust|GetGustPeriodA))) (Variables|Gust|GetGustAmpA)) (* (Math|Trig|Sin(Degrees) (/ (* _returnvalue_5 3.6e+02) (Variables|Gust|GetGustPeriodB))) (Variables|Gust|GetGustAmpB)) (* (Math|Trig|Sin(Degrees) (/ (* _returnvalue_5 3.6e+02) (Variables|Gust|GetGustPeriodC))) (Variables|Gust|GetGustAmpC))) 0.5) 0.5) (Variables|Gust|GetGustBias)) (* (Math|Float|Power (Math|Float|Max(Float) (Math|Trig|Sin(Degrees) (/ (* _returnvalue_5 3.6e+02) (Variables|Gust|GetPunchPeriod))) 0.0) (Variables|Gust|GetPunchPower)) (Variables|Gust|GetPunchAmount))))))