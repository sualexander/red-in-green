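; Free-fly debug pawn that visualizes the wind field around BP_Drone, with scroll-adjusted movement speed.
; Possession clears the post-process color grading LUT, plays a random click jingle and enables wind debug; unpossession undoes the visual changes.
; A toggleable looping timer samples BP_Wind on a layered grid, drawing arrows scaled and colored by strength, faded by distance from the pawn.
; It also draws labeled wind height bands at the drone.
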(event Custom|Jingle
  (Audio|PlaySound2D (.OutItem (Utilities|Array|Random (Utilities|Array|MakeArray "/Engine/VREditor/Sounds/VR_click1.VR_click1" "/Engine/VREditor/Sounds/VR_click2.VR_click2" "/Engine/VREditor/Sounds/VR_click3.VR_click3"))) (Math|Random|RandomFloatinRange 0.6 1.0) (Math|Random|RandomFloatinRange 0.8 1.2) 0.0 0 0)
  (if (Math|Random|RandomBoolwithWeight 0.92)
    (Utilities|FlowControl|Delay (Math|Random|RandomFloatinRange 0.1 0.4))
    (CallFunction|Jingle)))

(event Custom|ToggleWind
  (bind _droneref (Variables|Default|GetDroneRef)
    (:then
      (bind _isa (Utilities|FlowControl|FlipFlop)
        (:A
          (Variables|Default|SetbIsToggled _isa)
          (Rendering|SetVisibility (Variables|/Game/BP_Drone.BP_Drone_C|GetDebugMesh _droneref) true false)
          (bind _returnvalue (Utilities|Time|SetTimerbyEvent (delegate Custom|DebugTick) (Variables|Default|GetTickRate) true true))
          (bind _output_get (Variables|Default|SetDebugTickRef _returnvalue)))
        (:B
          (Variables|Default|SetbIsToggled _isa)
          (Rendering|SetVisibility (Variables|/Game/BP_Drone.BP_Drone_C|GetDebugMesh _droneref) false false)
          (Utilities|Time|ClearandInvalidateTimerbyHandle _output_get))))
    (:else)))

(event Custom|DebugTick
  (bind _windref (Variables|Default|GetWindRef))
  (bind _debugarea (Variables|Default|GetDebugArea))
  (bind _windref_2 (Variables|Default|GetWindRef))
  (bind _increment (Variables|Default|GetIncrement))
  (bind _returnvalue (* _debugarea -1))
  (bind _shelterheight (Variables|/Game/Wind/BP_Wind.BP_Wind_C|GetShelterHeight _windref_2))
  (Utilities|FlowControl|Sequence
    (:then_0
      (Variables|Default|SetTemp (* (+ (Variables|/Game/Wind/BP_Wind.BP_Wind_C|GetBaseSpeed _windref) (Variables|/Game/Wind/BP_Wind.BP_Wind_C|GetGustSpeed _windref)) (Variables|/Game/Wind/BP_Wind.BP_Wind_C|GetIntensityScale _windref)))
      (for _index (range 0 5)
        (for _index_2 (range _returnvalue _debugarea)
          (for _index_3 (range _returnvalue _debugarea)
            (Rendering|Debug|DrawDebugArrow (Math|Vector|MakeVector (.x (+ (Transformation|GetActorLocation (Variables|Default|GetDroneRef)) (Math|Vector|MakeVector (* _index_3 _increment) (* _index_2 _increment) 0.0))) (.y (+ (Transformation|GetActorLocation (Variables|Default|GetDroneRef)) (Math|Vector|MakeVector (* _index_3 _increment) (* _index_2 _increment) 0.0))) (+ (* _index 1000) 5e+02)) (+ (Math|Vector|MakeVector (.x (+ (Transformation|GetActorLocation (Variables|Default|GetDroneRef)) (Math|Vector|MakeVector (* _index_3 _increment) (* _index_2 _increment) 0.0))) (.y (+ (Transformation|GetActorLocation (Variables|Default|GetDroneRef)) (Math|Vector|MakeVector (* _index_3 _increment) (* _index_2 _increment) 0.0))) (+ (* _index 1000) 5e+02)) (* (Math|Vector|Normalize (Default|GetWindat (Variables|Default|GetWindRef) (Math|Vector|MakeVector (.x (+ (Transformation|GetActorLocation (Variables|Default|GetDroneRef)) (Math|Vector|MakeVector (* _index_3 _increment) (* _index_2 _increment) 0.0))) (.y (+ (Transformation|GetActorLocation (Variables|Default|GetDroneRef)) (Math|Vector|MakeVector (* _index_3 _increment) (* _index_2 _increment) 0.0))) (+ (* _index 1000) 5e+02)))) _increment (Math|Float|Clamp(Float) (/ (Math|Vector|VectorLength (Default|GetWindat (Variables|Default|GetWindRef) (Math|Vector|MakeVector (.x (+ (Transformation|GetActorLocation (Variables|Default|GetDroneRef)) (Math|Vector|MakeVector (* _index_3 _increment) (* _index_2 _increment) 0.0))) (.y (+ (Transformation|GetActorLocation (Variables|Default|GetDroneRef)) (Math|Vector|MakeVector (* _index_3 _increment) (* _index_2 _increment) 0.0))) (+ (* _index 1000) 5e+02)))) (Variables|Default|GetTemp))))) 6e+02 (Utilities|Struct|MakeLinearColor (.r (Math|Color|Lerp(LinearColor) "(R=0.000000,G=0.116786,B=1.000000,A=1.000000)" "(R=1.000000,G=0.020115,B=0.000000,A=1.000000)" (Math|Float|Clamp(Float) (/ (Math|Vector|VectorLength (Default|GetWindat (Variables|Default|GetWindRef) (Math|Vector|MakeVector (.x (+ (Transformation|GetActorLocation (Variables|Default|GetDroneRef)) (Math|Vector|MakeVector (* _index_3 _increment) (* _index_2 _increment) 0.0))) (.y (+ (Transformation|GetActorLocation (Variables|Default|GetDroneRef)) (Math|Vector|MakeVector (* _index_3 _increment) (* _index_2 _increment) 0.0))) (+ (* _index 1000) 5e+02)))) (Variables|Default|GetTemp))))) (.g (Math|Color|Lerp(LinearColor) "(R=0.000000,G=0.116786,B=1.000000,A=1.000000)" "(R=1.000000,G=0.020115,B=0.000000,A=1.000000)" (Math|Float|Clamp(Float) (/ (Math|Vector|VectorLength (Default|GetWindat (Variables|Default|GetWindRef) (Math|Vector|MakeVector (.x (+ (Transformation|GetActorLocation (Variables|Default|GetDroneRef)) (Math|Vector|MakeVector (* _index_3 _increment) (* _index_2 _increment) 0.0))) (.y (+ (Transformation|GetActorLocation (Variables|Default|GetDroneRef)) (Math|Vector|MakeVector (* _index_3 _increment) (* _index_2 _increment) 0.0))) (+ (* _index 1000) 5e+02)))) (Variables|Default|GetTemp))))) (.b (Math|Color|Lerp(LinearColor) "(R=0.000000,G=0.116786,B=1.000000,A=1.000000)" "(R=1.000000,G=0.020115,B=0.000000,A=1.000000)" (Math|Float|Clamp(Float) (/ (Math|Vector|VectorLength (Default|GetWindat (Variables|Default|GetWindRef) (Math|Vector|MakeVector (.x (+ (Transformation|GetActorLocation (Variables|Default|GetDroneRef)) (Math|Vector|MakeVector (* _index_3 _increment) (* _index_2 _increment) 0.0))) (.y (+ (Transformation|GetActorLocation (Variables|Default|GetDroneRef)) (Math|Vector|MakeVector (* _index_3 _increment) (* _index_2 _increment) 0.0))) (+ (* _index 1000) 5e+02)))) (Variables|Default|GetTemp))))) (- 1.0 (Math|Float|Clamp(Float) (/ (Math|Vector|Distance(Vector) (Math|Vector|MakeVector (.x (+ (Transformation|GetActorLocation (Variables|Default|GetDroneRef)) (Math|Vector|MakeVector (* _index_3 _increment) (* _index_2 _increment) 0.0))) (.y (+ (Transformation|GetActorLocation (Variables|Default|GetDroneRef)) (Math|Vector|MakeVector (* _index_3 _increment) (* _index_2 _increment) 0.0))) (+ (* _index 1000) 5e+02)) (Transformation|GetActorLocation)) 3e+04)))) (Variables|Default|GetTickRate) 8.0)))))
    (:then_1
      (CallFunction|HeightDebug (Variables|/Game/Wind/BP_Wind.BP_Wind_C|GetGroundZ _windref_2) _shelterheight "SPEED" "(R=0.135928,G=1.000000,B=0.000000,A=1.000000)")
      (CallFunction|HeightDebug _shelterheight (Variables|/Game/Wind/BP_Wind.BP_Wind_C|GetVeerHeight _windref_2) "DIRECTION" "(R=0.626253,G=1.000000,B=0.000000,A=1.000000)"))))

(event Custom|HeightDebug
  (params (Start :type Float%20%28double-precision%29) (End :type Float%20%28double-precision%29) (Text :type String) (LineColor :type Linear%20Color%20Structure))
  (bind _tickrate (Variables|Default|GetTickRate))
  (bind _droneref (Variables|Default|GetDroneRef))
  (bind _returnvalue (Transformation|GetActorLocation _droneref))
  (Rendering|Debug|DrawDebugLine (Math|Vector|MakeVector (.x _returnvalue) (.y _returnvalue) Start) (Math|Vector|MakeVector (.x _returnvalue) (.y _returnvalue) End) LineColor _tickrate 16.0 "Foreground")
  (Rendering|Debug|DrawDebugString (Math|Vector|MakeVector (+ (.x _returnvalue) 1e+02) (+ (.y _returnvalue) 1e+02) End) Text 0 LineColor _tickrate))

(event Input|EnhancedActionEvents|EnhancedInputActionIA_Debugs
  (params (ActionValue :type Float%20%28double-precision%29) (ElapsedSeconds :type Float%20%28double-precision%29) (TriggeredSeconds :type Float%20%28double-precision%29) (InputAction :type Input%20Action%20Object%20Reference :default "/Game/Input/IA_Debugs.IA_Debugs"))
  (:Started
    (switch int (Math|Float|Round ActionValue)
      (:2
        (CallFunction|ToggleWind)))))

(event Input|EnhancedActionEvents|EnhancedInputActionIA_Move
  (params (ActionValue :type Vector%202D%20Structure) (ElapsedSeconds :type Float%20%28double-precision%29) (TriggeredSeconds :type Float%20%28double-precision%29) (InputAction :type Input%20Action%20Object%20Reference :default "/Game/Input/IA_Move.IA_Move"))
  (Class|PawnMovementComponent|AddInputVector (Variables|Default|GetFloatingPawnMovement) (+ (* (.x ActionValue) (Transformation|GetActorRightVector)) (* (Transformation|GetActorForwardVector) (.y ActionValue))) false))

(event Input|EnhancedActionEvents|EnhancedInputActionIA_DebugQE
  (params (ActionValue :type Float%20%28double-precision%29) (ElapsedSeconds :type Float%20%28double-precision%29) (TriggeredSeconds :type Float%20%28double-precision%29) (InputAction :type Input%20Action%20Object%20Reference :default "/Game/Input/IA_DebugQE.IA_DebugQE"))
  (Class|PawnMovementComponent|AddInputVector (Variables|Default|GetFloatingPawnMovement) (Math|Vector|MakeVector 0.0 0.0 ActionValue) false))

(event Input|EnhancedActionEvents|EnhancedInputActionIA_Scroll
  (params (ActionValue :type Float%20%28double-precision%29) (ElapsedSeconds :type Float%20%28double-precision%29) (TriggeredSeconds :type Float%20%28double-precision%29) (InputAction :type Input%20Action%20Object%20Reference :default "/Game/Input/IA_Scroll.IA_Scroll"))
  (bind _floatingpawnmovement (Variables|Default|GetFloatingPawnMovement))
  (bind _returnvalue (Class|MovementComponent|GetMaxSpeed _floatingpawnmovement))
  (Variables|/Script/Engine.FloatingPawnMovement|SetMaxSpeed _floatingpawnmovement (Math|Float|Clamp(Float) (+ (* ActionValue 4.2e+02 (/ _returnvalue (Variables|Default|GetMaxSpeed))) _returnvalue) 8e+02 (Variables|Default|GetMaxSpeed))))

(event Input|EnhancedActionEvents|EnhancedInputActionIA_Look
  (params (ActionValue :type Vector%202D%20Structure) (ElapsedSeconds :type Float%20%28double-precision%29) (TriggeredSeconds :type Float%20%28double-precision%29) (InputAction :type Input%20Action%20Object%20Reference :default "/Game/Input/IA_Look.IA_Look"))
  (Pawn|Input|AddControllerYawInput (.x ActionValue))
  (Pawn|Input|AddControllerPitchInput (.y ActionValue)))

(event EventPossessed
  (params (NewController :type Controller%20Object%20Reference))
  (Utilities|FlowControl|Sequence
    (:then_0
      (bind _returnvalue (Actor|GetActorOfClass "/Script/Engine.PostProcessVolume"))
      (Utilities|IsValid _returnvalue
        (:Is%20Valid
          (Variables|Default|SetSaved (Utilities|Struct|BreakPostProcessSettings (Variables|/Script/Engine.PostProcessVolume|GetSettings _returnvalue)))
          (Utilities|Struct|SetmembersinPostProcessSettings (Variables|/Script/Engine.PostProcessVolume|GetSettings _returnvalue) 0))))
    (:then_1
      (CallFunction|Jingle)
      (Development|PrintString "- Debugging -"))
    (:then_2
      (bind _returnvalue_2 (Actor|GetActorOfClass "/Game/BP_Drone.BP_Drone_C"))
      (bind _output_get (Variables|Default|SetDroneRef _returnvalue_2))
      (Utilities|IsValid _output_get
        (:Is%20Valid
          (bind _returnvalue_3 (Actor|GetActorOfClass "/Game/Wind/BP_Wind.BP_Wind_C"))
          (Variables|Default|SetWindRef _returnvalue_3)
          (CallFunction|ToggleWind))))))

(event EventUnpossessed
  (params (OldController :type Controller%20Object%20Reference))
  (Utilities|FlowControl|Sequence
    (:then_0
      (bind _saved (Variables|Default|GetSaved)
        (:then
          (bind _returnvalue (Actor|GetActorOfClass "/Script/Engine.PostProcessVolume"))
          (Utilities|Struct|SetmembersinPostProcessSettings (Variables|/Script/Engine.PostProcessVolume|GetSettings _returnvalue) _saved))
        (:else)))
    (:then_1
      (Audio|PlaySound2D "/Engine/EditorSounds/GamePreview/EjectFromPlayer.EjectFromPlayer" 1.0 1.0 0.0 0 0)
      (Development|PrintString "- End Debugging -"))
    (:then_2
      (if (Variables|Default|GetbIsToggled)
        (CallFunction|ToggleWind)))))

(fn ConstructionScript)